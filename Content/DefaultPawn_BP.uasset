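; Default pawn Blueprint that lets the player interact with movable pictures by looking at them.
; On Interact, it line traces from the eye viewpoint along the view direction on the Visibility channel.
; A hit Movable_Picture_BP that has not yet spun is rotated by a timeline-driven pitch combined with its initial rotation.
; When the timeline finishes, the picture's HasSpined flag is set so it spins only once.
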(event Collision|EventActorBeginOverlap
  (params (OtherActor :type Actor%20Object%20Reference)))

(event EventTick
  (params (DeltaSeconds :type Float%20%28single-precision%29)))

(event Input|ActionEvents|InputActionInteract
  (params (Key :type Key%20Structure))
  (bind _returnvalue (Game|GetPlayerController 0))
  (bind (_outlocation _outrotation) (Actor|GetActorEyesViewPoint _returnvalue))
  (bind _returnvalue_2 (+ _outlocation "0, 0, 0"))
  (:Pressed
    (bind _outhit (Collision|LineTraceByChannel _returnvalue_2 (+ _returnvalue_2 (* (Math|Vector|GetForwardVector _outrotation) (Variables|Default|GetTraceLength))) "TraceTypeQuery1" false 0 "None"))
    (Utilities|IsValid (.hitactor _outhit)
      (:Is%20Valid
        (bind _asmovable_picture_bp (Utilities|Casting|CastToMovable_Picture_BP (.hitactor _outhit)))
        (if (not (Variables|/Game/Movable_Picture_BP.Movable_Picture_BP_C|GetHasSpined _asmovable_picture_bp))
          (Variables|Default|SetInitalPicRotation (Transformation|GetActorRotation _asmovable_picture_bp))
          (bind _newtrack_0 (Timeline|Timeline_0 Play)
            (:Update
              (Transformation|SetActorRotation _asmovable_picture_bp (Math|Rotator|CombineRotators (Math|Rotator|MakeRotator 0.0 _newtrack_0 0.0) (Variables|Default|GetInitalPicRotation))))
            (:Finished
              (Variables|/Game/Movable_Picture_BP.Movable_Picture_BP_C|SetHasSpined _asmovable_picture_bp true))))))))

(fn ConstructionScript)