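; Openable drawer actor that slides along the world Y axis when a DefaultPawn_BP overlaps it.
; BeginPlay stores the start location, and a timeline's Open curve offsets the drawer from it, reversing when any actor ends overlap.
; Each timeline update also adds a cumulative local Z offset to TargetActor, in both play directions.
; The OpenDrawer OnClose event is empty, and ActivateMessage is never run.
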(event OnClose(OpenDrawer))

(event EventBeginPlay
  (Variables|Default|SetInitial%20Position (Transformation|GetActorLocation)))

(event Collision|EventActorBeginOverlap
  (params (OtherActor :type Actor%20Object%20Reference))
  (Utilities|Casting|CastToDefaultPawn_BP OtherActor)
  (bind _open (Timeline|Timeline_0 Play)
    (:Update
      (Transformation|SetActorLocation (+ (Math|Vector|MakeVector 0.0 _open 0.0) (Variables|Default|GetInitial%20Position)) false false)
      (Transformation|AddActorLocalOffset (Variables|Default|GetTargetActor) "0, 0,100.000000" false false))))

(event Collision|EventActorEndOverlap
  (params (OtherActor :type Actor%20Object%20Reference))
  (bind _open (Timeline|Timeline_0 Reverse)
    (:Update
      (Transformation|SetActorLocation (+ (Math|Vector|MakeVector 0.0 _open 0.0) (Variables|Default|GetInitial%20Position)) false false)
      (Transformation|AddActorLocalOffset (Variables|Default|GetTargetActor) "0, 0,100.000000" false false))))

(fn ConstructionScript)