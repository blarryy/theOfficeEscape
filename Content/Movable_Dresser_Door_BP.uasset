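; Movable dresser door that swings open when the DefaultPawn_BP pawn overlaps it, also sliding a linked Desk actor.
; A timeline adds yaw to the rotation saved at BeginPlay.
; Its update plays a second timeline, if Desk is valid, that offsets the desk along world Y from its saved position.
; An event track on that timeline plays a music cue at the desk, and nothing reverses the motion on overlap end.
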(event EventBeginPlay
  (Variables|Default|SetInitial%20Rotation (Transformation|GetActorRotation))
  (Variables|Default|SetInitialDeskPosition (Transformation|GetActorLocation (Variables|Default|GetDesk))))

(event Collision|EventActorEndOverlap
  (params (OtherActor :type Actor%20Object%20Reference)))

(event EventTick
  (params (DeltaSeconds :type Float%20%28single-precision%29)))

(event Collision|EventActorBeginOverlap
  (params (OtherActor :type Actor%20Object%20Reference))
  (Utilities|Casting|CastToDefaultPawn_BP OtherActor)
  (bind _newtrack_0 (Timeline|Timeline_0 Play)
    (:Update
      (Transformation|SetActorRotation (Math|Rotator|CombineRotators (Math|Rotator|MakeRotator 0.0 0.0 _newtrack_0) (Variables|Default|GetInitial%20Rotation)))
      (Utilities|IsValid (Variables|Default|GetDesk)
        (:Is%20Valid
          (bind _newtrack_0_2 (Timeline|Timeline_1 Play)
            (:Update
              (Transformation|SetActorLocation (Variables|Default|GetDesk) (+ (Math|Vector|MakeVector 0.0 _newtrack_0_2 0.0) (Variables|Default|GetInitialDeskPosition)) false false))
            (:NewTrack_1
              (Audio|PlaySoundatLocation "/Game/StarterContent/Audio/Starter_Music_Cue.Starter_Music_Cue" (Transformation|GetActorLocation (Variables|Default|GetDesk)) "0, 0, 0" 1.0 1.0 0.0 0 0 0))))))))

(fn ConstructionScript)