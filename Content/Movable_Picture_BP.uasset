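; Movable picture Blueprint that slides a referenced dresser actor once its HasSpined flag is true.
; Tick checks the flag and plays a Timeline that offsets the dresser along Y from the location cached at BeginPlay.
; A Timeline event track spawns the Light01 2D sound and deactivates it after eight seconds.
; The flag is not set in this graph, and the MoveDresserSound playback is unconnected.
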(event EventBeginPlay
  (Variables|Default|SetInitialDresserLocation (Transformation|GetActorLocation (Variables|Default|GetMovable_Dresser))))

(event Collision|EventActorBeginOverlap
  (params (OtherActor :type Actor%20Object%20Reference)))

(event EventTick
  (params (DeltaSeconds :type Float%20%28single-precision%29))
  (if (Variables|Default|GetHasSpined)
    (Utilities|IsValid (Variables|Default|GetMovable_Dresser)
      (:Is%20Valid
        (bind _newtrack_0 (Timeline|Timeline_0 Play)
          (:Update
            (Transformation|SetActorLocation (Variables|Default|GetMovable_Dresser) (+ (Math|Vector|MakeVector 0.0 _newtrack_0 0.0) (Variables|Default|GetInitialDresserLocation)) false false))
          (:NewTrack_1
            (bind _returnvalue (Audio|SpawnSound2D "/Game/StarterContent/Audio/Light01.Light01" 1.0 1.0 0.0 0))
            (Utilities|FlowControl|Delay 8.0)
            (Components|Activation|SetActive _returnvalue false false)))))))

(fn ConstructionScript)