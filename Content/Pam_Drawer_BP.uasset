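; Pam's drawer actor, which slides open and closed through OpenDrawer and CloseDrawer events and sets off a cupboard move when first opened.
; Timelines offset the drawer along world Y from its position at the start of each move, with player input disabled until it finishes.
; After the first opening, a third timeline shifts MoveableCupboard once and its event track plays the Light01 sound, deactivated after a delay.
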(event Custom|OpenDrawer
  (Variables|Default|SetInitial%20Position (Transformation|GetActorLocation))
  (Input|DisableInput (Game|Player|GetPlayerPawn 0) 0)
  (bind _open (Timeline|Timeline_0 PlayFromStart)
    (:Update
      (Transformation|SetActorLocation (+ (Math|Vector|MakeVector 0.0 _open 0.0) (Variables|Default|GetInitial%20Position)) false false))
    (:Finished
      (Input|EnableInput (Game|Player|GetPlayerPawn 0) 0)
      (Variables|Default|SetPam_Drawer_IsOpen true)
      (if (not (Variables|Default|GetCupboard%20Is%20Moved))
        (bind _newtrack_0 (Timeline|Timeline_2 PlayFromStart)
          (:Update
            (Transformation|SetActorLocation (Variables|Default|GetMoveable_Cupboard) (+ (Math|Vector|MakeVector 0.0 _newtrack_0 0.0) (Variables|Default|GetInitial%20Cupboard%20Location%20)) false false))
          (:Finished
            (Variables|Default|SetCupboard%20Is%20Moved true))
          (:NewTrack_1
            (bind _returnvalue (Audio|SpawnSound2D "/Game/StarterContent/Audio/Light01.Light01" 1.0 1.0 0.0 0))
            (Utilities|FlowControl|Delay 8.0)
            (Components|Activation|SetActive _returnvalue false false)))))))

(event Custom|CloseDrawer
  (Variables|Default|SetInitial%20Position (Transformation|GetActorLocation))
  (Input|DisableInput (Game|Player|GetPlayerPawn 0) 0)
  (bind _open (Timeline|Timeline_1 PlayFromStart)
    (:Update
      (Transformation|SetActorLocation (+ (Math|Vector|MakeVector 0.0 _open 0.0) (Variables|Default|GetInitial%20Position)) false false))
    (:Finished
      (Input|EnableInput (Game|Player|GetPlayerPawn 0) 0)
      (Variables|Default|SetPam_Drawer_IsOpen false))))

(event EventBeginPlay
  (Variables|Default|SetPam_Drawer_IsOpen false)
  (Variables|Default|SetCupboard%20Is%20Moved false)
  (Variables|Default|SetInitial%20Cupboard%20Location%20 (Transformation|GetActorLocation (Variables|Default|GetMoveable_Cupboard))))

(event Collision|EventActorBeginOverlap
  (params (OtherActor :type Actor%20Object%20Reference)))

(event EventTick
  (params (DeltaSeconds :type Float%20%28single-precision%29)))

(fn ConstructionScript)